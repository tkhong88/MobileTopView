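; BP_Rifle is a rifle weapon that hands itself to a BP_CharacterFemaleA overlapping its Box and can snap-attach to a mesh socket.
; SetItemInfo loads weapon properties from DT_WeaponRifleInfo, using the item ID as row name.
; ApplyWeaponParam derives current spread from those properties, growing with the cube of ICount up to the maximum accuracy value.
; Tick eases spread back toward its initial value while TimeToDecay remains.
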(event `self.ReceiveTick`
  (params (DeltaSeconds :type "Float (single-precision)"))
  (if (and (> (`self.TimeToDecay`) 0.0) (> (`self.CurrentSpread`) (`self.InitialSpread`)))
    (set `self.CurrentSpread` (- (`self.CurrentSpread`) (* (- (`self.CurrentSpread`) (`self.InitialSpread`)) (`KismetMathLibrary.FMin` (/ DeltaSeconds (`self.TimeToDecay`)) 1.0))))
    (set `self.TimeToDecay` (`KismetMathLibrary.FMax` (- (`self.TimeToDecay`) DeltaSeconds)))))

(event `self.Box.OnComponentBeginOverlap`
  (params (OverlappedComponent :type "PrimitiveComponent Object Reference") (OtherActor :type "Actor Object Reference") (OtherComp :type "PrimitiveComponent Object Reference") (OtherBodyIndex :type Integer) (bFromSweep :type Boolean) (SweepResult :type "HitResult Structure (by ref)"))
  (`/Engine/EditorBlueprintResources/StandardMacros.IsValid` OtherActor
    (:`Is Valid`
      (bind _asbp_character_female_a (cast `/Game/TopDownCPP/Blueprints/BP_CharacterFemaleA` OtherActor))
      (`/Game/TopDownCPP/Blueprints/BP_CharacterFemaleA.SetWeapon` _asbp_character_female_a self))))

(event `self.SetItemInfo`
  (params (ItemInfo :type "StructMyItemInfo Structure"))
  (`parent.SetItemInfo` ItemInfo)
  (bind _returnvalue (`|GetDataTableRow` "/Game/Data/DT_WeaponRifleInfo.DT_WeaponRifleInfo" (`KismetStringLibrary.Conv_StringToName` (`KismetStringLibrary.Conv_IntToString` (`.ItemID` (break `StructMyItemInfo` ItemInfo)))))
    (:`then`
      (`self.SetWeaponProperty` (`.WeaponInfo_5_BB68FE3E4B8CA3BF37FB12B31EFAD861` (break `/Game/Data/structRifleInfo` _returnvalue))))))

(fn `ApplyWeaponParam`
  (bind _returnvalue (`self.GetWeaponProperty`))
  (bind (_initialaccuracy _maxaccuracy _increasingspeed) (break `structRifleSpreadInfo` (`.SpreadInfoSteady` (break `structRifleInfo` _returnvalue))))
  (set `self.InitialSpread` _initialaccuracy)
  (set `self.CurrentSpread` (`KismetMathLibrary.FMin` (+ (+ _initialaccuracy 1.0) (* (/ (- _maxaccuracy _initialaccuracy) (`KismetMathLibrary.MultiplyMultiply_FloatFloat` (`KismetMathLibrary.Conv_IntToDouble` _increasingspeed) 3.0)) (`KismetMathLibrary.MultiplyMultiply_FloatFloat` (`KismetMathLibrary.Conv_IntToDouble` (`self.iCount`)) 3.0))) _maxaccuracy))
  (set `self.isSpreadDecaying?` true))

(fn `Attach`
  (params (ParentMesh :type "SkeletalMeshComponent Object Reference") (SockName :type Name))
  (`self.K2_AttachToComponent` ParentMesh SockName "SnapToTarget" "KeepRelative" "KeepRelative"))

(fn `UserConstructionScript`)